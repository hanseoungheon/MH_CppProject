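; DinoValdo monster Blueprint that handles the creature's tail attack and death.
; Tail attack begin and end events switch four hit components between query-only collision and no collision.
; An overlap on any of them calls ApplyDamamge on the other actor with TailDMG and the monster's AI controller as instigator.
; MonsterDead stops the montage, prints a debug string and sets the monster state to Dead.
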(event `self.ReceiveBeginPlay`)

(event `self.MonsterDead`
  (`self.StopAnimMontage` null)
  (`KismetSystemLibrary.PrintString` "으앙쥬금")
  (`self.SetMonsterState` "Dead"))

(event `OnTailAttackBegin`
  (`PrimitiveComponent.SetCollisionEnabled` (`self.TailAttack1`) "QueryOnly")
  (`PrimitiveComponent.SetCollisionEnabled` (`self.TailAttack2`) "QueryOnly")
  (`PrimitiveComponent.SetCollisionEnabled` (`self.TailAttack3`) "QueryOnly")
  (`PrimitiveComponent.SetCollisionEnabled` (`self.TailAttack4`) "QueryOnly"))

(event `OnTailAttckEnd`
  (`PrimitiveComponent.SetCollisionEnabled` (`self.TailAttack1`) "NoCollision")
  (`PrimitiveComponent.SetCollisionEnabled` (`self.TailAttack2`) "NoCollision")
  (`PrimitiveComponent.SetCollisionEnabled` (`self.TailAttack3`) "NoCollision")
  (`PrimitiveComponent.SetCollisionEnabled` (`self.TailAttack4`) "NoCollision"))

(event `self.TailAttack1.OnComponentBeginOverlap`
  (params (OverlappedComponent :type "PrimitiveComponent Object Reference") (OtherActor :type "Actor Object Reference") (OtherComp :type "PrimitiveComponent Object Reference") (OtherBodyIndex :type Integer) (bFromSweep :type Boolean) (SweepResult :type "HitResult Structure (by ref)"))
  (`self.ApplyDamamge` OtherActor (`self.TailDMG`) (`AIBlueprintHelperLibrary.GetAIController` self)))

(event `self.TailAttack2.OnComponentBeginOverlap`
  (params (OverlappedComponent :type "PrimitiveComponent Object Reference") (OtherActor :type "Actor Object Reference") (OtherComp :type "PrimitiveComponent Object Reference") (OtherBodyIndex :type Integer) (bFromSweep :type Boolean) (SweepResult :type "HitResult Structure (by ref)"))
  (`self.ApplyDamamge` OtherActor (`self.TailDMG`) (`AIBlueprintHelperLibrary.GetAIController` self)))

(event `self.TailAttack3.OnComponentBeginOverlap`
  (params (OverlappedComponent :type "PrimitiveComponent Object Reference") (OtherActor :type "Actor Object Reference") (OtherComp :type "PrimitiveComponent Object Reference") (OtherBodyIndex :type Integer) (bFromSweep :type Boolean) (SweepResult :type "HitResult Structure (by ref)"))
  (`self.ApplyDamamge` OtherActor (`self.TailDMG`) (`AIBlueprintHelperLibrary.GetAIController` self)))

(event `self.TailAttack4.OnComponentBeginOverlap`
  (params (OverlappedComponent :type "PrimitiveComponent Object Reference") (OtherActor :type "Actor Object Reference") (OtherComp :type "PrimitiveComponent Object Reference") (OtherBodyIndex :type Integer) (bFromSweep :type Boolean) (SweepResult :type "HitResult Structure (by ref)"))
  (`self.ApplyDamamge` OtherActor (`self.TailDMG`) (`AIBlueprintHelperLibrary.GetAIController` self)))

(fn `UserConstructionScript`)