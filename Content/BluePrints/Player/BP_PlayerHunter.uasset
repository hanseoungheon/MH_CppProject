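; Player hunter Blueprint that equips the character with a hanging long sword and its housing.
; The SpawnLongSwordandHouse event spawns both actors, sets the player as their owner and stores references to them.
; Each actor snaps to its own socket on the player's Mesh.
; Tick prints IsCanAttack every frame as debug output, while BeginPlay, overlap and the construction script are empty.
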(event `self.ReceiveTick`
  (params (DeltaSeconds :type "Float (single-precision)"))
  (`KismetSystemLibrary.PrintString` (`KismetStringLibrary.Conv_BoolToString` (`self.bIsCanAttack`))))

(event `self.SpawnLongSwordAndHouse`
  (bind _returnvalue (`self.GetTransform`))
  (`|ExecutionSequence`
    (:`then_0`
      (bind _returnvalue_2 (`|SpawnActorFromClass` "/Game/BluePrints/Weapon/LongSword/Dummy/BP_HangingLongSword.BP_HangingLongSword_C" _returnvalue "Undefined" "MultiplyWithRoot" null null))
      (`MyDummyWeapon.MySetOwner` _returnvalue_2 self)
      (set `self.DummyLongSword` _returnvalue_2)
      (`self.K2_AttachToComponent` _returnvalue_2 (`self.Mesh`) "HaningLS" "SnapToTarget" "SnapToTarget" "SnapToTarget" true))
    (:`then_1`
      (bind _returnvalue_3 (`|SpawnActorFromClass` "/Game/BluePrints/Weapon/LongSword/Dummy/BP_LongSwordHouse.BP_LongSwordHouse_C" _returnvalue "Undefined" "MultiplyWithRoot" null null))
      (`MyDummyWeapon.MySetOwner` _returnvalue_3 self)
      (set `self.DummyLSHouse` _returnvalue_3)
      (`self.K2_AttachToComponent` _returnvalue_3 (`self.Mesh`) "LSHouse" "SnapToTarget" "SnapToTarget" "SnapToTarget" true))))

(fn `UserConstructionScript`)